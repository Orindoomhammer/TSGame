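; Base weapon actor that configures itself from a data table and fires projectiles automatically while the trigger is held.
; The construction script reads the hardcoded "Pistol" row for meshes, transform adjustments, damage, fire rate and projectile class.
; BeginPlay applies the meshes, rotation and offset.
; PullTrigger starts a looping timer that spawns projectiles at ProjectileSpawn, first after one interval, until ReleaseTrigger clears it.
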(event Custom|PullTrigger
  (bind _returnvalue (Utilities|Time|SetTimerbyEvent (delegate Custom|FireWeapon) (Variables|Default|GetFireRate) true)))

(event Custom|FireWeapon
  (Game|SpawnActorfromClass (Variables|Default|GetProjectileClass) (Transformation|GetWorldTransform (Variables|Default|GetProjectileSpawn)) "Undefined" 0 0))

(event Custom|ReleaseTrigger
  (Utilities|Time|ClearandInvalidateTimerbyHandle (stale Custom|PullTrigger _returnvalue)))

(event EventBeginPlay
  (bind _skeletalmesh (Variables|Default|GetSkeletalMesh))
  (Components|StaticMesh|SetStaticMesh (Variables|Default|GetStaticMesh) (Variables|Default|GetWeaponStMesh))
  (Class|SkinnedMeshComponent|SetSkeletalMesh (Variables|Default|GetSkeletalMesh) (Variables|Default|GetWeaponSkMesh) true)
  (Transformation|SetRelativeRotation _skeletalmesh (Variables|Default|GetWeaponRotation) false false)
  (Transformation|AddLocalOffset _skeletalmesh (Variables|Default|GetweaponOffset) false false))

(fn ConstructionScript
  (bind _returnvalue (Utilities|GetDataTableRow "/Game/TS_Blueprints/Data/DataTable/WeaponDataTable.WeaponDataTable" "Pistol")
    (:then
      (Variables|Default|SetWeaponName (.name _returnvalue))
      (Variables|Default|SetWeaponSkMesh (.sk_mesh _returnvalue))
      (Variables|Default|SetWeaponStMesh (.st_mesh _returnvalue))
      (Variables|Default|SetWeaponRotation (.weaponrotation _returnvalue))
      (Variables|Default|SetweaponOffset (.weaponoffset _returnvalue))
      (Variables|Default|SetDamage (.damage _returnvalue))
      (Variables|Default|SetFireRate (.fire_rate _returnvalue))
      (Variables|Default|SetProjectileClass (.projectileclass _returnvalue))
      (Class|SkinnedMeshComponent|SetSkeletalMesh (Variables|Default|GetSkeletalMesh) 0 true)
      (Components|StaticMesh|SetStaticMesh (Variables|Default|GetStaticMesh) 0))))